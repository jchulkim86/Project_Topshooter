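; Master modular zombie Blueprint that can randomize each zombie's look and animates its face with morph targets.
; With Randomize on, the construction script picks head, clothing, hair and materials from ModularVariations, plus per-instance gore masks that cost extra draw calls.
; Top and bottom meshes follow the body mesh through master pose.
; Every Tick, eye, snarl and mouth functions oscillate morph weights toward random peaks, choosing morph names by head type.
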(event EventBeginPlay
  (Class|SkeletalMeshComponent|ClearMorphTargets (Variables|Character|GetMesh))
  (Components|SkeletalMesh|SetMorphTarget (Variables|Character|GetMesh) "None" 0.0 true))

(event Collision|EventActorBeginOverlap
  (params (OtherActor :type Actor%20Object%20Reference)))

(event EventTick
  (params (DeltaSeconds :type Float%20%28single-precision%29))
  (CallFunction|EyeMovement 1.0)
  (CallFunction|SnarlMovement 1.0)
  (CallFunction|MouthMovement 1.0))

(fn ConstructionScript
  (bind _returnvalue (Math|Random|RandomFloatinRange 0.0 1.0))
  (bind _returnvalue_2 (Math|Random|RandomFloatinRange 0.0 1.0))
  (bind _returnvalue_3 (Math|Random|RandomInteger 4))
  (bind _mesh (Variables|Character|GetMesh))
  (bind _sk_top (Variables|Default|GetSK_Top))
  (bind _sk_top_2 (Variables|Default|GetSK_Top))
  (bind _modular_variations (Variables|Default|GetModular_Variations))
  (bind _sk_bottom (Variables|Default|GetSK_Bottom))
  (bind _sk_bottom_2 (Variables|Default|GetSK_Bottom))
  (bind _sm_hair (Variables|Default|GetSM_Hair))
  (bind _mesh_2 (Variables|Character|GetMesh))
  (bind (_tops _bottoms _head_accessories _zombie_types _limbs _heads _mi_longjeans _mi_singlet _mi_tshirt _mi_head01 _mi_head02 _mi_body _mi_haircolors) (Utilities|Struct|BreakStruc_ModularStarvedMaleVariations _modular_variations))
  (bind _returnvalue_4 (> _returnvalue_3 3))
  (Class|SkinnedMeshComponent|SetMasterPoseComponent (Variables|Default|GetSK_Top) (Variables|Character|GetMesh) false)
  (if (Variables|Default|GetRandomize?)
    (Variables|Default|SetRandomBodyType (Math|Random|RandomInteger (Utilities|Array|Length _mi_body)))
    (Utilities|FlowControl|Sequence
      (:then_0
        ;[1 1 1] Randomize Hair Color
        (Rendering|Material|SetMaterial (Variables|Default|GetSM_Hair) 1 (Utilities|Array|Get(acopy) _mi_haircolors (Math|Random|RandomInteger (Utilities|Array|Length _mi_haircolors)))))
      (:then_1
        ;[1 1 1] Randomize Shirt/Singlet
        (if _returnvalue_4
          (Rendering|SetVisibility _sk_top_2 false false)
          (else
            (Class|SkinnedMeshComponent|SetSkeletalMesh _sk_top_2 (Utilities|Array|Get(acopy) _tops (Math|Random|RandomInteger (Utilities|Array|Length _tops))) true)
            (if (Utilities|String|Contains (Utilities|GetDisplayName _sk_top_2) "singlet")
              (Rendering|Material|SetMaterial _sk_top_2 0 (Utilities|Array|Get(acopy) _mi_singlet (Math|Random|RandomInteger (Utilities|Array|Length _mi_singlet))))
              (else
                (Rendering|Material|SetMaterial _sk_top_2 0 (Utilities|Array|Get(acopy) _mi_tshirt (Math|Random|RandomInteger (Utilities|Array|Length _mi_tshirt))))))
            (Rendering|SetVisibility _sk_top_2 true false))))
      (:then_2
        ;[1 1 1] RandomizePants
        (if _returnvalue_4
          (Rendering|SetVisibility _sk_bottom_2 false false)
          (else
            (Class|SkinnedMeshComponent|SetSkeletalMesh _sk_bottom_2 (Utilities|Array|Get(acopy) _bottoms (Math|Random|RandomInteger (Utilities|Array|Length _bottoms))) true)
            (Rendering|SetVisibility _sk_bottom_2 true false)
            (Rendering|Material|SetMaterial _sk_bottom_2 0 (Utilities|Array|Get(acopy) _mi_longjeans (Math|Random|RandomInteger (Utilities|Array|Length _mi_longjeans))))
            (Rendering|SetVisibility _sk_bottom_2 true false))))
      (:then_3
        ;[1 1 1] Randomize Head Type and Zombie Skin
        (Class|SkinnedMeshComponent|SetSkeletalMesh _mesh (Utilities|Array|Get(acopy) _zombie_types (Math|Random|RandomInteger (Utilities|Array|Length _zombie_types))) true)
        (Rendering|Material|SetMaterialbyName _mesh "Body" (Utilities|Array|Get(acopy) _mi_body (Variables|Default|GetRandomBodyType)))
        (if (> (Math|Random|RandomInteger 2) 0)
          (Rendering|SetVisibility _sm_hair false false)
          (else
            (Rendering|SetVisibility _sm_hair true false)))
        (if (Utilities|String|Contains (Utilities|GetDisplayName _mesh) "_02")
          (Rendering|Material|SetMaterialbyName _mesh "Head" (Utilities|Array|Get(acopy) _mi_head02 (Math|Random|RandomInteger (Utilities|Array|Length _mi_head02))))
          (else
            (Rendering|Material|SetMaterialbyName _mesh "Head" (Utilities|Array|Get(acopy) _mi_head01 (Math|Random|RandomInteger (Utilities|Array|Length _mi_head01)))))))
      (:then_4
        ;[1 1 1] Warning: This can greatly increase draw calls/material count, but randomizes the gore masks for every zombie spawned. It makes each material instance unique and no longer instancable
        (Rendering|Material|SetScalarParameterValueonMaterials _sk_bottom "6.Mask_1" _returnvalue_2)
        (Rendering|Material|SetScalarParameterValueonMaterials _sk_bottom "7.Mask_2" _returnvalue_2)
        (Rendering|Material|SetScalarParameterValueonMaterials _sk_bottom "8.Mask_3" _returnvalue_2)
        (Rendering|Material|SetScalarParameterValueonMaterials _sk_bottom "9.Mask_4" _returnvalue_2)
        (Rendering|Material|SetScalarParameterValueonMaterials _sk_top "6.Mask_1" _returnvalue)
        (Rendering|Material|SetScalarParameterValueonMaterials _sk_top "7.Mask_2" _returnvalue)
        (Rendering|Material|SetScalarParameterValueonMaterials _sk_top "8.Mask_3" _returnvalue)
        (Rendering|Material|SetScalarParameterValueonMaterials _sk_top "9.Mask_4" _returnvalue)
        (Rendering|Material|SetScalarParameterValueonMaterials _mesh_2 "6.Mask_1" 0.0)
        (Rendering|Material|SetScalarParameterValueonMaterials _mesh_2 "7.Mask_2" 0.0)
        (Rendering|Material|SetScalarParameterValueonMaterials _mesh_2 "8.Mask_3" 0.0)))))

(fn EyeMovement
  (params (EyeMovementSpeed :type Float%20%28single-precision%29))
  (bind _mesh (Variables|Character|GetMesh))
  (Utilities|FlowControl|Sequence
    (:then_0
      (if (Variables|FacialControl|Eyes|GetChangeDirection)
        (Utilities|FlowControl|Sequence
          (:then_0
            (Variables|FacialControl|Eyes|SetEyeMax (Math|Random|RandomFloatinRange (Variables|FacialControl|Eyes|GetRandomLowEye) (Variables|FacialControl|Eyes|GetRandomHighEye)))
            (Variables|FacialControl|Eyes|SetForward (not (Variables|FacialControl|Eyes|GetForward)))
            (Variables|FacialControl|Eyes|SetChangeDirection false))
          (:then_1
            (if (Variables|FacialControl|Eyes|GetForward)
              (Variables|FacialControl|Eyes|SetToZero false)
              (if (> (Variables|FacialControl|Eyes|GetMorphMovementSpeed_Eyes) 0.0)
                (Variables|FacialControl|Eyes|SetMorphMovementSpeed_Eyes (Variables|FacialControl|Eyes|GetMorphMovementSpeed_Eyes))
                (else
                  (bind _result (Math|Float|NegateFloat (Variables|FacialControl|Eyes|GetMorphMovementSpeed_Eyes))
                    (:%20%20
                      (Variables|FacialControl|Eyes|SetMorphMovementSpeed_Eyes _result)))))
              (else
                (Variables|FacialControl|Eyes|SetToZero true)
                (if (< (Variables|FacialControl|Eyes|GetMorphMovementSpeed_Eyes) 0.0)
                  (Variables|FacialControl|Eyes|SetMorphMovementSpeed_Eyes (Variables|FacialControl|Eyes|GetMorphMovementSpeed_Eyes))
                  (else
                    (bind _result_2 (Math|Float|NegateFloat (Variables|FacialControl|Eyes|GetMorphMovementSpeed_Eyes))
                      (:%20%20
                        (Variables|FacialControl|Eyes|SetMorphMovementSpeed_Eyes _result_2)))))))))))
    (:then_1
      (if (Variables|FacialControl|Eyes|GetToZero)
        (if (> (Variables|FacialControl|Eyes|GetEyeLeftRight%20Amount) 0.0)
          (Variables|FacialControl|Eyes|SetEyeLeftRight%20Amount (Math|Float|Clamp(Float) (* (+ (Variables|FacialControl|Eyes|GetEyeLeftRight%20Amount) (Variables|FacialControl|Eyes|GetMorphMovementSpeed_Eyes)) EyeMovementSpeed)))
          (if (Variables|FacialControl|Eyes|GetBlendToNewMorph) :!label _label
            (Components|SkeletalMesh|SetMorphTarget _mesh "R_Eye_Right" (stale _output_get) true)
            (Components|SkeletalMesh|SetMorphTarget _mesh "L_Eye_Right" (stale _output_get) true)
            (else
              (Components|SkeletalMesh|SetMorphTarget _mesh "R_Eye_Left" (stale _output_get) true)
              (Components|SkeletalMesh|SetMorphTarget _mesh "L_Eye_Left" (stale _output_get) true)))
          (else
            (Variables|FacialControl|Eyes|SetBlendToNewMorph (not (Variables|FacialControl|Eyes|GetBlendToNewMorph)))
            (Variables|FacialControl|Eyes|SetChangeDirection true)))
        (else
          (bind _output_get (Variables|FacialControl|Eyes|SetEyeLeftRight%20Amount (Math|Float|Clamp(Float) (* (+ (Variables|FacialControl|Eyes|GetEyeLeftRight%20Amount) (Variables|FacialControl|Eyes|GetMorphMovementSpeed_Eyes)) EyeMovementSpeed))))
          (if (> _output_get (Variables|FacialControl|Eyes|GetEyeMax))
            (Variables|FacialControl|Eyes|SetChangeDirection true)
            (else
              (goto _label))))))))

(fn SnarlMovement
  (params (EyeMovementSpeed :type Float%20%28single-precision%29))
  (bind _mesh (Variables|Character|GetMesh))
  (Utilities|FlowControl|Sequence
    (:then_0
      (if (Variables|FacialControl|Snarl|GetChangeDirection_Snarl)
        (Utilities|FlowControl|Sequence
          (:then_0
            (Variables|FacialControl|Snarl|SetSnarl_Max (Math|Random|RandomFloatinRange (Variables|FacialControl|Snarl|GetRandomLowSnarl) (Variables|FacialControl|Snarl|GetRandomHighSnarl)))
            (Variables|FacialControl|Snarl|SetForward_Snarl (not (Variables|FacialControl|Snarl|GetForward_Snarl)))
            (Variables|FacialControl|Snarl|SetChangeDirection_Snarl false))
          (:then_1
            (if (Variables|FacialControl|Snarl|GetForward_Snarl)
              (Variables|FacialControl|Snarl|SetToZero_Snarl false)
              (if (> (Variables|FacialControl|Snarl|GetMorphMovementSpeed_Snarl) 0.0)
                (Variables|FacialControl|Snarl|SetMorphMovementSpeed_Snarl (Variables|FacialControl|Snarl|GetMorphMovementSpeed_Snarl))
                (else
                  (bind _result (Math|Float|NegateFloat (Variables|FacialControl|Snarl|GetMorphMovementSpeed_Snarl))
                    (:%20%20
                      (Variables|FacialControl|Snarl|SetMorphMovementSpeed_Snarl _result)))))
              (else
                (Variables|FacialControl|Snarl|SetToZero_Snarl true)
                (if (< (Variables|FacialControl|Snarl|GetMorphMovementSpeed_Snarl) 0.0)
                  (Variables|FacialControl|Snarl|SetMorphMovementSpeed_Snarl (Variables|FacialControl|Snarl|GetMorphMovementSpeed_Snarl))
                  (else
                    (bind _result_2 (Math|Float|NegateFloat (Variables|FacialControl|Snarl|GetMorphMovementSpeed_Snarl))
                      (:%20%20
                        (Variables|FacialControl|Snarl|SetMorphMovementSpeed_Snarl _result_2)))))))))))
    (:then_1
      (if (Variables|FacialControl|Snarl|GetToZero_Snarl)
        (if (> (Variables|FacialControl|Snarl|GetSnarl_Amount) 0.0)
          (Variables|FacialControl|Snarl|SetSnarl_Amount (Math|Float|Clamp(Float) (* (+ (Variables|FacialControl|Snarl|GetSnarl_Amount) (Variables|FacialControl|Snarl|GetMorphMovementSpeed_Snarl)) EyeMovementSpeed)))
          (if (Utilities|String|Contains (Utilities|GetDisplayName _mesh) "_02") :!label _label
            (Components|SkeletalMesh|SetMorphTarget _mesh "Snarl_B" (stale _output_get) true)
            (else
              (Components|SkeletalMesh|SetMorphTarget _mesh "Snarl_A" (stale _output_get) true)))
          (else
            (Variables|FacialControl|Snarl|SetChangeDirection_Snarl true)))
        (else
          (bind _output_get (Variables|FacialControl|Snarl|SetSnarl_Amount (Math|Float|Clamp(Float) (* (+ (Variables|FacialControl|Snarl|GetSnarl_Amount) (Variables|FacialControl|Snarl|GetMorphMovementSpeed_Snarl)) EyeMovementSpeed))))
          (if (> _output_get (Variables|FacialControl|Snarl|GetSnarl_Max))
            (Variables|FacialControl|Snarl|SetChangeDirection_Snarl true)
            (else
              (goto _label))))))))

(fn MouthMovement
  (params (EyeMovementSpeed :type Float%20%28single-precision%29))
  (bind _mesh (Variables|Character|GetMesh))
  (Utilities|FlowControl|Sequence
    (:then_0
      (if (Variables|FacialControl|Mouth|GetChangeDirection_Mouth)
        (Utilities|FlowControl|Sequence
          (:then_0
            (Variables|FacialControl|Mouth|SetMouth_Max (Math|Random|RandomFloatinRange (Variables|FacialControl|Mouth|GetRandomLow_Mouth) (Variables|FacialControl|Mouth|GetRandomHigh_Mouth)))
            (Variables|FacialControl|Mouth|SetForward_Mouth (not (Variables|FacialControl|Mouth|GetForward_Mouth)))
            (Variables|FacialControl|Mouth|SetChangeDirection_Mouth false))
          (:then_1
            (if (Variables|FacialControl|Mouth|GetForward_Mouth)
              (Variables|FacialControl|Mouth|SetToZero_Mouth false)
              (if (> (Variables|FacialControl|Mouth|GetMorphMovementSpeed_Mouth) 0.0)
                (Variables|FacialControl|Mouth|SetMorphMovementSpeed_Mouth (Variables|FacialControl|Mouth|GetMorphMovementSpeed_Mouth))
                (else
                  (bind _result (Math|Float|NegateFloat (Variables|FacialControl|Mouth|GetMorphMovementSpeed_Mouth))
                    (:%20%20
                      (Variables|FacialControl|Mouth|SetMorphMovementSpeed_Mouth _result)))))
              (else
                (Variables|FacialControl|Mouth|SetToZero_Mouth true)
                (if (< (Variables|FacialControl|Mouth|GetMorphMovementSpeed_Mouth) 0.0)
                  (Variables|FacialControl|Mouth|SetMorphMovementSpeed_Mouth (Variables|FacialControl|Mouth|GetMorphMovementSpeed_Mouth))
                  (else
                    (bind _result_2 (Math|Float|NegateFloat (Variables|FacialControl|Mouth|GetMorphMovementSpeed_Mouth))
                      (:%20%20
                        (Variables|FacialControl|Mouth|SetMorphMovementSpeed_Mouth _result_2)))))))))))
    (:then_1
      (if (Variables|FacialControl|Mouth|GetToZero_Mouth)
        (if (> (Variables|FacialControl|Mouth|GetMouth_Amount) 0.0)
          (Variables|FacialControl|Mouth|SetMouth_Amount (Math|Float|Clamp(Float) (* (+ (Variables|FacialControl|Mouth|GetMouth_Amount) (Variables|FacialControl|Mouth|GetMorphMovementSpeed_Mouth)) EyeMovementSpeed)))
          (if (Utilities|String|Contains (Utilities|GetDisplayName _mesh) "_02") :!label _label
            (Components|SkeletalMesh|SetMorphTarget _mesh "MouthControl_B" (stale _output_get) true)
            (else
              (Components|SkeletalMesh|SetMorphTarget _mesh "MouthControl_A" (stale _output_get) true)))
          (else
            (Variables|FacialControl|Mouth|SetChangeDirection_Mouth true)))
        (else
          (bind _output_get (Variables|FacialControl|Mouth|SetMouth_Amount (Math|Float|Clamp(Float) (* (+ (Variables|FacialControl|Mouth|GetMouth_Amount) (Variables|FacialControl|Mouth|GetMorphMovementSpeed_Mouth)) EyeMovementSpeed))))
          (if (> _output_get (Variables|FacialControl|Mouth|GetMouth_Max))
            (Variables|FacialControl|Mouth|SetChangeDirection_Mouth true)
            (else
              (goto _label))))))))