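; BP_LimbSpawner is an actor that repeatedly spawns physics-driven zombie limbs at its own transform.
; Tick feeds a Delay of SpawnFrequency, which acts as a repeating timer for spawning BP_LimbSpawnerSelector actors.
; Each limb's SKLimb gets physics-only collision, simulation and a random impulse that launches it upward with sideways scatter.
; The spawner passes its DestroyTime to each spawned actor.
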(event EventBeginPlay)

(event Collision|EventActorBeginOverlap
  (params (OtherActor :type Actor%20Object%20Reference)))

(event EventTick
  (params (DeltaSeconds :type Float%20%28single-precision%29))
  (bind _returnvalue (Math|Random|RandomFloatinRange -2.5e+02 2.5e+02))
  (Utilities|FlowControl|Delay (Variables|Default|GetSpawnFrequency))
  (bind _returnvalue_2 (Game|SpawnActorfromClass "/Game/ETC/YI_ModularZombies/Blueprints/ZombieM02/ZombieLimbPhysicsSpawner/BP_LimbSpawnerSelector.BP_LimbSpawnerSelector_C" (Transformation|GetActorTransform self) "Undefined" 0 0))
  (Collision|SetCollisionEnabled (Variables|/Game/ETC/YI_ModularZombies/Blueprints/ZombieM02/ZombieLimbPhysicsSpawner/BP_LimbSpawnerSelector.BP_LimbSpawnerSelector_C|GetSK_Limb _returnvalue_2) "PhysicsOnly")
  (Physics|SetSimulatePhysics (Variables|/Game/ETC/YI_ModularZombies/Blueprints/ZombieM02/ZombieLimbPhysicsSpawner/BP_LimbSpawnerSelector.BP_LimbSpawnerSelector_C|GetSK_Limb _returnvalue_2) true)
  (Physics|AddImpulse (Variables|/Game/ETC/YI_ModularZombies/Blueprints/ZombieM02/ZombieLimbPhysicsSpawner/BP_LimbSpawnerSelector.BP_LimbSpawnerSelector_C|GetSK_Limb _returnvalue_2) (Math|Vector|MakeVector _returnvalue _returnvalue (Math|Random|RandomFloatinRange 5e+02 7.5e+02)) "None" false)
  (Variables|/Game/ETC/YI_ModularZombies/Blueprints/ZombieM02/ZombieLimbPhysicsSpawner/BP_LimbSpawnerSelector.BP_LimbSpawnerSelector_C|SetDestroyTime _returnvalue_2 (Variables|Default|GetDestroyTime)))

(fn ConstructionScript)